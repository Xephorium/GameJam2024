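; Box puzzle actor that is solved when the overlapping actor touches all eight of its colliders at once.
; Begin overlap stores any entering actor as Player and sets a flag, which end overlap clears.
; While flagged, Tick tests every collider against that actor through a Gate.
; On success it plays a victory sound, activates the PExplosion effect and closes the gate to stop further checks.
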(event EventTick
  (params (DeltaSeconds :type Float%20%28single-precision%29))
  (bind _player (Variables|Default|GetPlayer))
  (Utilities|FlowControl|Gate false :!label _label
    (:Exit
      (if (Variables|Default|GetbIsOverlappingPlayer)
        (if (Math|Boolean|ANDBoolean (Collision|IsOverlappingActor (Variables|Default|GetColliders3) _player :!class /Script/Engine.PrimitiveComponent) (Collision|IsOverlappingActor (Variables|Default|GetColliders2) _player :!class /Script/Engine.PrimitiveComponent) (Collision|IsOverlappingActor (Variables|Default|GetColliders6) _player :!class /Script/Engine.PrimitiveComponent) (Collision|IsOverlappingActor (Variables|Default|GetColliders1) _player :!class /Script/Engine.PrimitiveComponent) (Collision|IsOverlappingActor (Variables|Default|GetColliders4) _player :!class /Script/Engine.PrimitiveComponent) (Collision|IsOverlappingActor (Variables|Default|GetColliders7) _player :!class /Script/Engine.PrimitiveComponent) (Collision|IsOverlappingActor (Variables|Default|GetColliders) _player :!class /Script/Engine.PrimitiveComponent) (Collision|IsOverlappingActor (Variables|Default|GetColliders5) _player :!class /Script/Engine.PrimitiveComponent))
          (Audio|PlaySoundatLocation "/Game/Audio/FF7_Victory.FF7_Victory" (Transformation|GetActorLocation) "0, 0, 0" 1.0 1.0 0.0 0 0 0 0)
          (Components|Activation|Activate (Variables|Default|GetP_Explosion) false)
          (goto _label Close))))))

(event Collision|EventActorBeginOverlap
  (params (OtherActor :type Actor%20Object%20Reference))
  (Variables|Default|SetbIsOverlappingPlayer true)
  (Variables|Default|SetPlayer OtherActor))

(event Collision|EventActorEndOverlap
  (params (OtherActor :type Actor%20Object%20Reference))
  (Variables|Default|SetbIsOverlappingPlayer false))

(fn ConstructionScript)